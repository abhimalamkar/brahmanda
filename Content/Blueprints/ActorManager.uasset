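; ActorManager is an actor that spawns and moves NPC personas as directed by a Socket.IO server.
; On connection it emits "init" and binds events: "some" spawns a named BP_ThirdPersonNPC per persona at its own transform, filling a name-to-actor map.
; Each "act" message supplies per-persona movement coordinates, scaled by 100 and passed to that NPC's MoveTo.
; SendPerception serializes a perception struct to JSON and emits it as "percive".
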(event OnConnected(SocketIOClient)
  (params (SocketId :type String) (SessionId :type String) (bIsReconnection :type Boolean))
  (bind _socketioclient (Variables|Default|GetSocketIOClient))
  (Class|SocketIOClientComponent|BindEventtoFunction _socketioclient "act" "PerformAct" 0 "/" "USE_DEFAULT")
  (Development|PrintString SessionId)
  (Class|SocketIOClientComponent|Emit _socketioclient "init" (Class|SIOJsonValue|ConstructJsonValueString "Hello There!") "/")
  (Class|SocketIOClientComponent|BindEventtoFunction _socketioclient "some" "ActionInit" 0 "/" "USE_DEFAULT")
  (Development|PrintString "Hello"))

(event Custom|ActionInit
  (params (Message :type SIO%20Json%20Value%20Object%20Reference))
  (for _array_element (Class|SIOJsonValue|AsArray (Class|SIOJsonObject|GetField (Class|SIOJLibrary|ToJsonObject(JsonValue) Message) "personas"))
    (bind _returnvalue (Game|SpawnActorfromClass "/Game/ThirdPerson/Blueprints/BP_ThirdPersonNPC.BP_ThirdPersonNPC_C" (Transformation|GetActorTransform) "Undefined" "MultiplyWithRoot" 0 0))
    (Variables|/Game/ThirdPerson/Blueprints/BP_ThirdPersonNPC.BP_ThirdPersonNPC_C|SetName _returnvalue (Class|SIOJsonValue|AsString _array_element))
    (Utilities|Map|Add (Variables|Default|Getactors) (Class|SIOJsonValue|AsString _array_element) _returnvalue)
    (Utilities|Array|AppendArray (Variables|Default|Getpersonas) (Utilities|Array|MakeArray (Class|SIOJsonValue|AsString _array_element)))))

(event Custom|PerformAct
  (params (Message :type SIO%20Json%20Value%20Object%20Reference))
  (for _array_element (Variables|Default|Getpersonas)
    (bind _returnvalue (Class|SIOJsonObject|GetNumberArrayField (Class|SIOJLibrary|ToJsonObject(JsonValue) (Class|SIOJsonObject|GetField (Class|SIOJLibrary|ToJsonObject(JsonValue) (Class|SIOJsonObject|GetField (Class|SIOJLibrary|ToJsonObject(JsonValue) Message) "persona")) _array_element)) "movement"))
    (Default|Moveto (.Value (Utilities|Map|Find (Variables|Default|Getactors) _array_element)) (Math|Vector|MakeVector (* (Utilities|Array|Get(acopy) _returnvalue) 1e+02) (* (Utilities|Array|Get(acopy) _returnvalue 1) 1e+02) 0.0))
    (Development|PrintString "Hello")))

(event EventBeginPlay)

(event Collision|EventActorBeginOverlap
  (params (OtherActor :type Actor%20Object%20Reference)))

(event EventTick
  (params (DeltaSeconds :type Float%20%28single-precision%29)))

(event EventSendPerception
  (params (Perception :type Event%20Structure))
  (Class|SocketIOClientComponent|Emit (Variables|Default|GetSocketIOClient) "percive" (Class|SIOJLibrary|ToJsonValue(JsonObject) (Class|SIOJLibrary|StructtoJsonObject Perception)) "/"))

(fn ConstructionScript)